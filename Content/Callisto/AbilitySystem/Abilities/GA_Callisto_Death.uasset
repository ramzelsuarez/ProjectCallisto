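; Gameplay ability that handles a Callisto character's death and respawn.
; On activation it plays a death montage and applies a death gameplay effect, then respawns when the montage completes, is interrupted or is cancelled.
; Respawn removes the Dead status effect, has the server reset attributes and move the character to a player start, calls the character's respawn handler, then ends the ability.
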(event `self.K2_ActivateAbility`
  (bind _returnvalue (`self.GetAbilitySystemComponentFromActorInfo`))
  (`AbilityTask_PlayMontageAndWait.CreatePlayMontageAndWaitProxy` "None" (`self.DeathMontage`)
    (:`then`
      ;[0.007269 0.01903 0.15 0.5] Applies the Dead Tag
      (`AbilitySystemComponent.BP_ApplyGameplayEffectSpecToSelf` _returnvalue (`AbilitySystemComponent.MakeOutgoingSpec` :`self` _returnvalue :`GameplayEffectClass` "/Game/Callisto/AbilitySystem/GameplayEffects/GE_Death.GE_Death_C" :`Level` 1.0)))
    (:`OnCompleted`
      (`self.RespawnCharacter` :!label _label))
    (:`OnInterrupted`
      (goto _label))
    (:`OnCancelled`
      (goto _label))))

(event `RespawnCharacter`
  (`|ExecutionSequence`
    (:`then_0`
      (`self.BP_RemoveGameplayEffectFromOwnerWithGrantedTags` (struct :`GameplayTags` (struct :`(TagName` "CallistoTags.Status.Dead"))) 1))
    (:`then_1`
      ;[0.007269 0.01903 0.15 0.5] Cache Callisto Base Character
      (bind _ascallisto_base_character (cast `Callisto_BaseCharacter` (`self.GetAvatarActorFromActorInfo`)))
      (set `self.CallistoBaseCharacter` _ascallisto_base_character))
    (:`then_2`
      ;[0.15 0.01548 0.01118 0.5] Server Only
      (`self.K2_HasAuthority`
        (:`True`
          (`|ExecutionSequence`
            (:`then_0`
              ;;[0.007269 0.01903 0.15 0.5] Reset Attributes
              (bind _callistobasecharacter (`self.CallistoBaseCharacter`)
                (:`then`
                  (`Callisto_BaseCharacter.ResetAttributes` _callistobasecharacter))
                (:`else`)))
            (:`then_1`
              ;;[0.007269 0.01903 0.15 0.5] "Respawning" the character
              (bind _callistobasecharacter_2 (`self.CallistoBaseCharacter`)
                (:`then`
                  (`Actor.K2_SetActorLocation` (`self.CallistoBaseCharacter`) (`Actor.K2_GetActorLocation` (`GameModeBase.K2_FindPlayerStart` (`GameplayStatics.GetGameMode`) (`Pawn.GetController` _callistobasecharacter_2) "")) false false))
                (:`else`)))))))
    (:`then_3`
      ;[0.007269 0.01903 0.15 0.5] Handle Respawn
      (bind _callistobasecharacter_3 (`self.CallistoBaseCharacter`)
        (:`then`
          (`Callisto_BaseCharacter.HandleRespawn` _callistobasecharacter_3))
        (:`else`)))
    (:`then_4`
      (`self.K2_EndAbility`))))