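; Gameplay ability for Callisto that watches its owner's health and triggers death when it reaches zero or below.
; On activation it starts a ListenForAttributeChange async task on the owner's ability system component and stores it, ending it when the ability ends.
; Each change optionally prints the new value for debugging, and depleted health activates abilities by the Death tag, allowing remote activation.
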(event `self.K2_ActivateAbility`
  (bind (_asynctaskproxy _attribute _newvalue) (`Callisto_AttributeChangeTask.ListenForAttributeChange` (`self.GetAbilitySystemComponentFromActorInfo`) (struct :`AttributeName` "Health" :`Attribute` "/Script/ProjectCallisto.Callisto_AttributeSet:Health" :`AttributeOwner` "/Script/CoreUObject.Class'/Script/ProjectCallisto.Callisto_AttributeSet'"))
    (:`then`
      (set `self.AttributeChangeTask` _asynctaskproxy))
    (:`OnAttributeChanged`
      (`self.DebugPrintNewHealth` _newvalue)
      (if (<= _newvalue 0.0)
        (`AbilitySystemComponent.TryActivateAbilitiesByTag` (`self.GetAbilitySystemComponentFromActorInfo`) (`BlueprintGameplayTagLibrary.MakeGameplayTagContainerFromTag` (`BlueprintGameplayTagLibrary.MakeLiteralGameplayTag` (struct :`TagName` "CallistoTags.CallistoAbilities.Death"))) true)))))

(event `self.K2_OnEndAbility`
  (params (bWasCancelled :type Boolean))
  (bind _attributechangetask (`self.AttributeChangeTask`)
    (:`then`
      (`Callisto_AttributeChangeTask.EndTask` _attributechangetask))
    (:`else`)))

(fn `DebugPrintNewHealth`
  (params (InDouble :type "Float (double-precision)"))
  (`self.bDrawDebugs`
    (:`then`
      (`KismetSystemLibrary.PrintString` (`KismetStringLibrary.Concat_StrStr` "GA_Callisto_ListenForHealthChange for:" (`KismetSystemLibrary.GetDisplayName` (`self.GetAvatarActorFromActorInfo`)) (`KismetStringLibrary.Conv_DoubleToString` InDouble))))
    (:`else`)))