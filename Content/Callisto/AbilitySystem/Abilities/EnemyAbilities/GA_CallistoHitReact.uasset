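; Enemy gameplay ability for Callisto that plays a directional hit reaction when the avatar is hit.
; On activation it waits for the HitReact gameplay event, then caches direction vectors from the event's instigator.
; The hit direction, derived from avatar forward and the vector to the instigator, becomes a section name that the hit react montage jumps to.
; Optional debug prints show the instigator and direction.
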(event `self.K2_ActivateAbility`
  (bind (_asynctaskproxy _payload) (`AbilityTask_WaitGameplayEvent.WaitGameplayEvent` (struct :`TagName` "CallistoTags.Events.Enemy.HitReact") null)
    (:`EventReceived`
      (`self.PrintDebugEventReceived` _payload)
      (`self.CacheDirectionVectors` (`.Instigator` (break `GameplayEventData` _payload)))
      (`|ExecutionSequence`
        (:`then_0`
          ;[0.007269 0.01903 0.15 0.5] Cache Hit Direction Name
          (set `self.HitDirectionName` (`Callisto_BlueprintLibrary.GetHitDirectionName` (`Callisto_BlueprintLibrary.GetHitDirection` (`self.AvatarForward`) (`self.ToInstigator`))))
          ;[0.15 0.01548 0.01118 0.5] Debug for Hit Direction
          (`self.bDrawDebugs`
            (:`then`
              (`KismetSystemLibrary.PrintString` (`KismetStringLibrary.Conv_NameToString` (`self.HitDirectionName`))))
            (:`else`)))
        (:`then_1`
          ;[0.007269 0.01903 0.15 0.5] Play Montage and Jump to the correct Hit React Montage Section
          (`AbilityTask_PlayMontageAndWait.CreatePlayMontageAndWaitProxy` "None" (`self.HitReactMontage`)
            (:`then`
              (`self.MontageJumpToSection` (`self.HitDirectionName`)))))))))

(fn `PrintDebugEventReceived`
  (params (GameplayEventData :type "GameplayEventData Structure (by ref)"))
  (`self.bDrawDebugs`
    (:`then`
      (`KismetSystemLibrary.PrintString` (`KismetStringLibrary.Concat_StrStr` "GA_Callisto_HitReact Received Event from:" (`KismetSystemLibrary.GetDisplayName` (`.Instigator` (break `GameplayEventData` GameplayEventData)))) true true (struct :`R` 1.0 :`G` 0.015625 :`B` 0.936368 :`A` 1.0)))
    (:`else`)))