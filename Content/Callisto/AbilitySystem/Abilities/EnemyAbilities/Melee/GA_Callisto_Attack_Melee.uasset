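; Enemy melee attack gameplay ability for Callisto.
; On activation it plays a random attack montage and ends when that completes, is interrupted or is cancelled, then sends an EndAttack event to the avatar.
; In parallel it waits for one MeleeTraceHit gameplay event and draws a debug sphere at the impact point.
; The SendDamageEventToPlayer call is disconnected, so this graph sends no damage.
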(event `self.K2_ActivateAbility`
  (`|ExecutionSequence`
    (:`then_0`
      ;[0.007269 0.01903 0.15 0.5] Play Attack Montage
      (`AbilityTask_PlayMontageAndWait.CreatePlayMontageAndWaitProxy` "None" (`KismetArrayLibrary.Array_Random` (`self.AttackMontages`))
        (:`OnCompleted`
          _)
        (:`OnInterrupted`
          _)
        (:`OnCancelled`
          _))
      (`self.K2_EndAbility`))
    (:`then_1`
      (bind (_asynctaskproxy _payload) (`AbilityTask_WaitGameplayEvent.WaitGameplayEvent` (struct :`TagName` "CallistoTags.Events.Enemy.MeleeTraceHit") null true)
        (:`EventReceived`
          (bind (_returnvalue_bblockinghit _returnvalue_binitialoverlap _returnvalue_time _returnvalue_distance _returnvalue_location _returnvalue_impactpoint) (`GameplayStatics.BreakHitResult` (`AbilitySystemBlueprintLibrary.EffectContextGetHitResult` (`.ContextHandle` (break `GameplayEventData` _payload)))))
          (`KismetSystemLibrary.DrawDebugSphere` _returnvalue_impactpoint 25.0 12 (struct :`R` 0.157735 :`G` 1.0 :`B` 0.142839 :`A` 1.0) 5.0))))))

(event `self.K2_OnEndAbility`
  (params (bWasCancelled :type Boolean))
  (`AbilitySystemBlueprintLibrary.SendGameplayEventToActor` (`self.GetAvatarActorFromActorInfo`) (struct :`TagName` "CallistoTags.Events.Enemy.EndAttack")))