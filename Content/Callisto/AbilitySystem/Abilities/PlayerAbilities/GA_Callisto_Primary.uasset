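; GA_Callisto_Primary is the player's primary attack gameplay ability for Callisto.
; On activation a FlipFlop alternates between two attack montages, ending the ability when the montage completes, blends out or is interrupted or cancelled.
; In parallel it waits for the Primary gameplay event, runs a hitbox overlap test, sends hit-react events and applies GE_PlayerDamage at ability level to each overlapped actor.
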(event `self.K2_ActivateAbility`
  (bind _returnvalue (`self.GetAbilitySystemComponentFromActorInfo`))
  (`|ExecutionSequence`
    (:`then_0`
      ;[0.05076 0.07912 0.15 0.5] Play Attack Montage
      (`/Engine/EditorBlueprintResources/StandardMacros.FlipFlop`
        (:`A`
          (`AbilityTask_PlayMontageAndWait.CreatePlayMontageAndWaitProxy` "None" "/Game/Callisto/Characters/PlayerCharacter/Animations/Callisto_Primary_A_Montage.Callisto_Primary_A_Montage"
            (:`OnCompleted`
              _)
            (:`OnBlendOut`
              _)
            (:`OnInterrupted`
              _)
            (:`OnCancelled`
              _))
          (`self.K2_EndAbility`))
        (:`B`
          (`AbilityTask_PlayMontageAndWait.CreatePlayMontageAndWaitProxy` "None" "/Game/Callisto/Characters/PlayerCharacter/Animations/Callisto_Primary_B_Montage.Callisto_Primary_B_Montage"
            (:`OnCompleted`
              _)
            (:`OnBlendOut`
              _)
            (:`OnInterrupted`
              _)
            (:`OnCancelled`
              _))
          (`self.K2_EndAbility`))))
    (:`then_1`
      (`AbilityTask_WaitGameplayEvent.WaitGameplayEvent` (struct :`TagName` "CallistoTags.Events.Player.Primary") null
        (:`EventReceived`
          (bind _returnvalue_2 (`self.HitBoxOverlapTest`))
          (`self.SendHitReactEventToActors` _returnvalue_2)
          (for _array_element _returnvalue_2
            (`AbilitySystemComponent.BP_ApplyGameplayEffectSpecToTarget` _returnvalue (`AbilitySystemComponent.MakeOutgoingSpec` :`self` _returnvalue :`GameplayEffectClass` "/Game/Callisto/AbilitySystem/GameplayEffects/Player/GE_PlayerDamage.GE_PlayerDamage_C" :`Level` (`KismetMathLibrary.Conv_IntToDouble` (`self.GetAbilityLevel`))) (`AbilitySystemBlueprintLibrary.GetAbilitySystemComponent` _array_element))))))))

(event `self.K2_OnEndAbility`
  (params (bWasCancelled :type Boolean))
  (if (`self.bDrawDebugs`)
    (`KismetSystemLibrary.PrintString` "GA_Primary: ENDED")))