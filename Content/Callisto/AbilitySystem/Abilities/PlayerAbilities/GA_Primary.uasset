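; GA_Primary is Callisto's primary ability, a Gameplay Ability that plays her primary montage.
; On each activation a FlipFlop alternates between the A and B montages, played through a play-montage-and-wait task.
; The ability ends when the montage completes, blends out, is interrupted or is cancelled, with optional debug prints on start and end.
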(event `self.K2_ActivateAbility`
  (if (`self.bDrawDebugs`)
    (`KismetSystemLibrary.PrintString` "GA_Primary: ACTIVATED"))
  (`/Engine/EditorBlueprintResources/StandardMacros.FlipFlop`
    (:`A`
      (`AbilityTask_PlayMontageAndWait.CreatePlayMontageAndWaitProxy` "None" "/Game/Callisto/Characters/PlayerCharacter/Animations/Callisto_Primary_A_Montage.Callisto_Primary_A_Montage"
        (:`OnCompleted`
          _)
        (:`OnBlendOut`
          _)
        (:`OnInterrupted`
          _)
        (:`OnCancelled`
          _))
      (`self.K2_EndAbility`))
    (:`B`
      (`AbilityTask_PlayMontageAndWait.CreatePlayMontageAndWaitProxy` "None" "/Game/Callisto/Characters/PlayerCharacter/Animations/Callisto_Primary_B_Montage.Callisto_Primary_B_Montage"
        (:`OnCompleted`
          _)
        (:`OnBlendOut`
          _)
        (:`OnInterrupted`
          _)
        (:`OnCancelled`
          _))
      (`self.K2_EndAbility`))))

(event `self.K2_OnEndAbility`
  (params (bWasCancelled :type Boolean))
  (if (`self.bDrawDebugs`)
    (`KismetSystemLibrary.PrintString` "GA_Primary: ENDED")))