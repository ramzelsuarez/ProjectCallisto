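; Callisto's primary attack gameplay ability, which plays a melee montage and tests for hits.
; A FlipFlop alternates between the A and B attack montages, and the ability ends when the montage completes, blends out, is interrupted or is cancelled.
; In parallel it waits for the Primary player gameplay event and runs a hit box overlap test when that event arrives.
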(event `self.K2_ActivateAbility`
  (`self.bDrawDebugs`
    (:`then`
      (`KismetSystemLibrary.PrintString` "GA_Primary: ACTIVATED"))
    (:`else`
      _))
  (`|ExecutionSequence`
    (:`then_0`
      ;[0.05076 0.07912 0.15 0.5] Play Attack Montage
      (`/Engine/EditorBlueprintResources/StandardMacros.FlipFlop`
        (:`A`
          (`AbilityTask_PlayMontageAndWait.CreatePlayMontageAndWaitProxy` "None" "/Game/Callisto/Characters/PlayerCharacter/Animations/Callisto_Primary_A_Montage.Callisto_Primary_A_Montage"
            (:`OnCompleted`
              _)
            (:`OnBlendOut`
              _)
            (:`OnInterrupted`
              _)
            (:`OnCancelled`
              _))
          (`self.K2_EndAbility`))
        (:`B`
          (`AbilityTask_PlayMontageAndWait.CreatePlayMontageAndWaitProxy` "None" "/Game/Callisto/Characters/PlayerCharacter/Animations/Callisto_Primary_B_Montage.Callisto_Primary_B_Montage"
            (:`OnCompleted`
              _)
            (:`OnBlendOut`
              _)
            (:`OnInterrupted`
              _)
            (:`OnCancelled`
              _))
          (`self.K2_EndAbility`))))
    (:`then_1`
      (`AbilityTask_WaitGameplayEvent.WaitGameplayEvent` (struct :`TagName` "CallistoTags.Events.Player.Primary") null
        (:`EventReceived`
          (`self.HitBoxOverlapTest`))))))

(event `self.K2_OnEndAbility`
  (params (bWasCancelled :type Boolean))
  (if (`self.bDrawDebugs`)
    (`KismetSystemLibrary.PrintString` "GA_Primary: ENDED")))